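; BP_LaneSpawner is a spawner actor that creates BP_Lane actors, starting at the player pawn's location on BeginPlay.
; SpawnLane records the newest lane and gives it a reference back to the spawner.
; A startup loop calls SpawnLaneAtSpawnPoint once a lane exists, but that function is empty.
; Its logic for chaining lanes at the newest lane's SpawnPoint is disconnected, so no further lanes spawn.
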(event `self.ReceiveBeginPlay`
  (`self.SpawnInitialLanes`))

(fn `SpawnInitialLanes`
  (for _ (range 3)
    (`/Engine/EditorBlueprintResources/StandardMacros.IsValid` (`self.NewestLane`)
      (:`Is Valid`
        (`self.SpawnLaneAtSpawnPoint`))
      (:`Is Not Valid`
        (`self.SpawnLane` (`self.K2_GetActorLocation` (`GameplayStatics.GetPlayerPawn` 0)))))))

(fn `SpawnLane`
  (params (SpawnLocation :type "Vector Structure"))
  (bind _returnvalue (`|SpawnActorFromClass` "/Game/Blueprints/BP_Lane.BP_Lane_C" (`KismetMathLibrary.MakeTransform` SpawnLocation) "Undefined" "OverrideRootScale" null null))
  (bind _output_get (set `self.NewestLane` _returnvalue))
  (set `/Game/Blueprints/BP_Lane.LaneSpawner` self _output_get))

(fn `SpawnLaneAtSpawnPoint`)

(fn `UserConstructionScript`)