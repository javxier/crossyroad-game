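; BP_Lane is a highway lane segment that replaces itself as the player moves along.
; When BP_Player overlaps TriggerZone, it tells LaneSpawner to spawn a lane at the spawn point, then destroys itself.
; RandomizeLane gives WallMesh a random marked or unmarked one-lane highway mesh, but nothing in this Blueprint calls it.
; The Tick rotation of WallMesh multiplies by zero, so it has no effect, and RotateSpeed is unused.
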(event `self.ReceiveTick`
  (params (DeltaSeconds :type "Float (single-precision)"))
  (`SceneComponent.K2_AddLocalRotation` (`self.WallMesh`) (`KismetMathLibrary.MakeRotator` (* DeltaSeconds 0.0)) false false))

(event `self.TriggerZone.OnComponentBeginOverlap`
  (params (OverlappedComponent :type "PrimitiveComponent Object Reference") (OtherActor :type "Actor Object Reference") (OtherComp :type "PrimitiveComponent Object Reference") (OtherBodyIndex :type Integer) (bFromSweep :type Boolean) (SweepResult :type "HitResult Structure (by ref)"))
  (cast `/Game/Blueprints/BP_Player` OtherActor)
  (`/Game/Blueprints/BP_LaneSpawner.SpawnLaneAtSpawnPoint` (`self.LaneSpawner`))
  (`self.K2_DestroyActor`))

(fn `RandomizeLane`
  (`StaticMeshComponent.SetStaticMesh` (`self.WallMesh`) (select `int` (`KismetMathLibrary.RandomIntegerInRange` 0 3) :`0` "/Game/Objects/Lanes/1lane_highway_marked.1lane_highway_marked" :`1` "/Game/Objects/Lanes/1lane_highway_unmarked.1lane_highway_unmarked" :`2` "/Game/Objects/Lanes/1lane_highway_marked.1lane_highway_marked" :`3` "/Game/Objects/Lanes/1lane_highway_unmarked.1lane_highway_unmarked" :!type "StaticMesh Object Reference")))

(fn `UserConstructionScript`)